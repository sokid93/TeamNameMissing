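; GridActor is a single grid tile that reacts to overlaps according to its tile type: Normal, Obstacle, Enemy or Collectible.
; On BeginPlay it caches BP_Player and GridControl; box overlaps, unfiltered by actor, call AplicarRaiz on the player for Enemy tiles.
; Collectible overlaps raise the player's score and have GridControl move the final tile.
; EventChangeType swaps the mesh material by type, with Obstacle sharing the Normal material.
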(event OnComponentBeginOverlap(BoxCollision)
  (params (OverlappedComponent :type Primitive%20Component%20Object%20Reference) (OtherActor :type Actor%20Object%20Reference) (OtherComp :type Primitive%20Component%20Object%20Reference) (OtherBodyIndex :type Integer) (bFromSweep :type Boolean) (SweepResult :type Hit%20Result%20Structure%20%28by%20ref%29))
  ;[1 1 1] Call effect when BP_Player falls on Collectible or Enemy Tile
  (switch Utilities|FlowControl|Switch|SwitchonTileState (Utilities|Enum|ByteToEnumTileState (Variables|Default|GetType))
    (:NewEnumerator2
      (Default|AplicarRaiz (Variables|Default|GetPlayerReference)))
    (:NewEnumerator3
      (Default|AumentarPuntuacion (Variables|Default|GetPlayerReference))
      (Default|ChangeFinalTilePos (Variables|Default|GetGridControlRef)))))

(event Custom|EventChangeType
  ;[1 1 1] Set Tile material depending on type
  (switch Utilities|FlowControl|Switch|SwitchonTileState (Utilities|Enum|ByteToEnumTileState (Variables|Default|GetType))
    (:NewEnumerator0
      (Rendering|Material|SetMaterial (Variables|Default|GetStaticMesh) 0 "/Game/Assets_Julia/Materials/NormalTile.NormalTile"))
    (:NewEnumerator1
      (Rendering|Material|SetMaterial (Variables|Default|GetStaticMesh) 0 "/Game/Assets_Julia/Materials/NormalTile.NormalTile"))
    (:NewEnumerator2
      (Rendering|Material|SetMaterial (Variables|Default|GetStaticMesh) 0 "/Game/Assets_Julia/Materials/EnemyTile.EnemyTile"))
    (:NewEnumerator3
      (Rendering|Material|SetMaterial (Variables|Default|GetStaticMesh) 0 "/Game/Assets_Julia/Materials/FinalTile.FinalTile"))))

(event EventBeginPlay
  ;[1 1 1] Get references to Actor_Player and Actor_GridControl
  (bind _returnvalue (Actor|GetActorOfClass "/Game/Blueprints/BP_Player.BP_Player_C"))
  (Variables|Default|SetPlayerReference _returnvalue)
  (bind _returnvalue_2 (Actor|GetActorOfClass "/Game/Assets_Julia/Blueprints/GridControl.GridControl_C"))
  (Variables|Default|SetGridControlRef _returnvalue_2))

(fn ConstructionScript)