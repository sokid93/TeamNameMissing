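; Grid manager that spawns a floor of GridActor tiles at BeginPlay and controls a randomly jumping enemy tile.
; Tiles and their locations are stored in flat arrays, with computed indices setting the initial enemy and final tiles.
; StartEnemyEvent starts a looping timer that moves the enemy to a random index, excluding the final tile.
; Each move restores the previous tile's saved type and triggers EventChangeType on affected tiles.
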(event Custom|StartEnemyEvent
  ;[1 1 1] Enemy Movement Trigger
  (Utilities|Time|SetTimerbyFunctionName 0 "EnemyMovement" 0.75 true))

(event EventBeginPlay
  ;[1 1 1] Create Grid Loop
  ;;[1 1 1] Generate X,Y indexes
  (for _index (range 0 (- (Variables|Components|GetGridX) 1))
    (for _index_2 (range 0 (- (Variables|Components|GetGridY) 1))
      ;;[1 1 1] Use Indexes to spawn and place floor tiles
      (bind _returnvalue (Game|SpawnActorfromClass "/Game/Assets_Julia/Blueprints/GridActor.GridActor_C" (Math|Transform|MakeTransform (Math|Vector|MakeVector (Math|Conversions|ToFloat(Integer) (* _index (Variables|Components|GetTileSize))) (Math|Conversions|ToFloat(Integer) (* _index_2 (Variables|Components|GetTileSize))) 0.0)) "Undefined" 0 0))
      ;;[1 1 1] Store each actor location in array
      (Utilities|Array|Add (Variables|Components|GetLocationOfTilesInWorld) (+ (.Location (Math|Transform|BreakTransform (Math|Transform|MakeTransform (Math|Vector|MakeVector (Math|Conversions|ToFloat(Integer) (* _index (Variables|Components|GetTileSize))) (Math|Conversions|ToFloat(Integer) (* _index_2 (Variables|Components|GetTileSize))) 0.0)))) (Variables|Components|GetInitialWorldPositionOfGrid)))
      ;;[1 1 1] Create array of grid actors
      (Utilities|Array|Add (Variables|Components|GetGridActorMatrix) _returnvalue)))
  ;[1 1 1] Set Initial Enemy Position and Final Tile
  (CallFunction|SetInitialEventTilesPositions))

(fn ConstructionScript
  ;[1 1 1] Init Variables
  (Variables|Components|SetTileLocationIndex 0)
  (Variables|Components|SetTileActorIndex 0)
  (Variables|Components|SetNumberOfTiles (* (Variables|Components|GetGridX) (Variables|Components|GetGridY)))
  ;[1 1 1] Clear location array
  (Utilities|Array|Clear (Variables|Components|GetLocationOfTilesInWorld))
  ;[1 1 1] Clear Actors array
  (Utilities|Array|Clear (Variables|Components|GetGridActorMatrix)))

(fn SetInitialEventTilesPositions
  ;[1 1 1] Define initial Enemy position
  (Variables|Components|SetEnemyActorIndex (- (Variables|Components|GetNumberOfTiles) (Variables|Components|GetGridX)))
  ;[1 1 1] Define Final position
  (Variables|Components|SetEndGameActorIndex (- (Variables|Components|GetNumberOfTiles) 1))
  ;[1 1 1] Set Final Tile
  (bind _output_get (Variables|Components|SetCurrentTile (Utilities|Array|Get(acopy) (Variables|Components|GetGridActorMatrix) (Variables|Components|GetEndGameActorIndex))))
  (bind _asgrid_actor (Utilities|Casting|CastToGridActor _output_get))
  (Variables|/Game/Assets_Julia/Blueprints/GridActor.GridActor_C|SetType _asgrid_actor (Variables|Components|GetTILE_TYPE_FINAL))
  (Default|EventChangeType _asgrid_actor)
  ;[1 1 1] Set Enemy Tile
  (bind _output_get_2 (Variables|Components|SetCurrentTile (Utilities|Array|Get(acopy) (Variables|Components|GetGridActorMatrix) (Variables|Components|GetEnemyActorIndex))))
  (bind _asgrid_actor_2 (Utilities|Casting|CastToGridActor _output_get_2))
  (Variables|/Game/Assets_Julia/Blueprints/GridActor.GridActor_C|SetType _asgrid_actor_2 (Variables|Components|GetTILE_TYPE_ENEMY))
  (Default|EventChangeType _asgrid_actor_2)
  ;[1 1 1] Update OldIndex value
  (Variables|Components|SetEnemyPreviousActorIndex (Variables|Components|GetEnemyActorIndex)))

(fn EnemyMovement
  ;[1 1 1] Set Enemy next destination, avoiding Final tile
  (Variables|Components|SetEnemyActorIndex (Math|Random|RandomIntegerinRange 0 (- (Variables|Components|GetNumberOfTiles) 2)))
  (CallFunction|SetTiletoEnemy))

(fn SetTiletoEnemy
  ;[1 1 1] Set previous ENEMY tile to previous type value.
  (CallFunction|SetTiletoPreviousType)
  ;[1 1 1] Store the current value of the future Enemy tile as OldType
  (bind _output_get (Variables|Components|SetCurrentTile (Utilities|Array|Get(acopy) (Variables|Components|GetGridActorMatrix) (Variables|Components|GetEnemyActorIndex))))
  (bind _asgrid_actor (Utilities|Casting|CastToGridActor _output_get))
  (Variables|Components|SetEnemyPreviousType (Variables|/Game/Assets_Julia/Blueprints/GridActor.GridActor_C|GetType _asgrid_actor))
  ;[1 1 1] Change the grid type and trigger the event
  (bind _output_get_2 (Variables|Components|SetCurrentTile (Utilities|Array|Get(acopy) (Variables|Components|GetGridActorMatrix) (Variables|Components|GetEnemyActorIndex))))
  (bind _asgrid_actor_2 (Utilities|Casting|CastToGridActor _output_get_2))
  (Variables|/Game/Assets_Julia/Blueprints/GridActor.GridActor_C|SetType _asgrid_actor_2 (Variables|Components|GetTILE_TYPE_ENEMY))
  (Default|EventChangeType _asgrid_actor_2)
  ;[1 1 1] Update OldIndex value
  (Variables|Components|SetEnemyPreviousActorIndex (Variables|Components|GetEnemyActorIndex)))

(fn SetTiletoPreviousType
  ;[1 1 1] This function is used ONLY for reseting the Enemy tile!!!
  (bind _output_get (Variables|Components|SetCurrentTile (Utilities|Array|Get(acopy) (Variables|Components|GetGridActorMatrix) (Variables|Components|GetEnemyPreviousActorIndex))))
  (bind _asgrid_actor (Utilities|Casting|CastToGridActor _output_get))
  (Variables|/Game/Assets_Julia/Blueprints/GridActor.GridActor_C|SetType _asgrid_actor (Variables|Components|GetEnemyPreviousType))
  (Default|EventChangeType _asgrid_actor))