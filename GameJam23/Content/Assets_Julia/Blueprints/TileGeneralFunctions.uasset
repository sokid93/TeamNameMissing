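; Tile helper function library for a grid-based game with enemies, collectibles and obstacles.
; Converts between X/Y and flat array indices, and saves, sets or reverts tile types, firing each tile's change event on set and revert.
; Spawn or movement pickers return random indices: odd for enemies, even for collectibles, or any from an allowed list.
; A filter builds that kind of list by excluding obstacle indices, and a debug helper prints arrays.
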(fn PrintArray
  (params (toPrint :type Array%20of%20Integers))
  (for _array_element toPrint
    (LocalVariables|SetarrayString (Utilities|String|Append (LocalVariables|GetarrayString) (Utilities|String|ToString(Integer) _array_element) ",")))
  (Development|PrintString 0 (Utilities|String|Append (LocalVariables|GetarrayString) "]") true true "(R=0.000000,G=0.660000,B=1.000000,A=1.000000)" 1e+01))

(fn GetTileVectorIndex
  (params (X :type Integer) (Y :type Integer) (SideOfTiles :type Integer))
  (return (+ X (* Y SideOfTiles))))

(fn GetTileMatrixIndex
  (params (VectorIndex :type Integer) (SideOfTiles :type Integer))
  (return (Math|Integer|%(Integer) VectorIndex SideOfTiles) (/ VectorIndex SideOfTiles)))

(fn RevertTiletoPrevType
  (params (TileToUpdate :type Grid%20Actor%20Object%20Reference))
  (Variables|/Game/Assets_Julia/Blueprints/GridActor.GridActor_C|SetType TileToUpdate (Variables|/Game/Assets_Julia/Blueprints/GridActor.GridActor_C|GetPastType TileToUpdate))
  (Default|EventChangeType TileToUpdate))

(fn SetTiletoNewType
  (params (TileToChange :type Grid%20Actor%20Object%20Reference) (NewType :type Byte))
  (Variables|/Game/Assets_Julia/Blueprints/GridActor.GridActor_C|SetType TileToChange NewType)
  (Default|EventChangeType TileToChange))

(fn EnemyBehavior1
  (params (NumberOfTiles :type Integer))
  (LocalVariables|SetNewEnemyIndex (Math|Random|RandomIntegerinRange 0 (- NumberOfTiles 1)))
  (if (== (Math|Integer|%(Integer) (LocalVariables|GetNewEnemyIndex) 2) 0)
    (LocalVariables|SetNewEnemyIndex (+ (LocalVariables|GetNewEnemyIndex) 1)))
  (return (LocalVariables|GetNewEnemyIndex)))

(fn RandomTileBehavior1
  (params (AllowedTiles :type Array%20of%20Integers))
  (bind _output_get (LocalVariables|SetNewEnemyIndex (Utilities|Array|Get(acopy) AllowedTiles (Math|Random|RandomIntegerinRange 0 (- (Utilities|Array|Length AllowedTiles) 1)))))
  (return _output_get))

(fn SaveOldTileType
  (params (Tile :type Grid%20Actor%20Object%20Reference))
  (Variables|/Game/Assets_Julia/Blueprints/GridActor.GridActor_C|SetPastType Tile (Variables|/Game/Assets_Julia/Blueprints/GridActor.GridActor_C|GetType Tile)))

(fn CollectibleBehavior1
  (params (NumberOfTiles :type Integer))
  (LocalVariables|SetNewCollectibleIndex (Math|Random|RandomIntegerinRange 0 (- NumberOfTiles 1)))
  (if (== (Math|Integer|%(Integer) (LocalVariables|GetNewCollectibleIndex) 2) 1)
    (LocalVariables|SetNewCollectibleIndex (- (LocalVariables|GetNewCollectibleIndex) 1)))
  (return (LocalVariables|GetNewCollectibleIndex)))

(fn GetAllowedTilesforMovement
  (params (ObstacleIndexes :type Array%20of%20Integers) (TotalTiles :type Integer))
  (LocalVariables|Setobstacles ObstacleIndexes)
  ;[1 1 1] Fill the Array with indexes that are NOT in the obstacle array
  (for _index (range 0 TotalTiles)
    (if (not (Utilities|Array|ContainsItem (LocalVariables|Getobstacles) _index))
      (Utilities|Array|Add (LocalVariables|Getindexes) _index)))
  (return (LocalVariables|Getindexes)))