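; Player for a grid puzzle game about square numbers, moving a cube tile by tile and showing its points on three text renders.
; Directional inputs step a flat index through GridControl's tile array, once per press, with modulo checks preventing row wrap.
; AumentarPuntuacion raises perfect squares to the next square and squares other values.
; AplicarRaiz takes the square root, but non-square points kill the player, triggering fade-out and game-over widgets.
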(event Custom|Aplicar%20Raiz
  (if (== (Math|Float|Fraction (Math|Float|Sqrt (Math|Conversions|ToFloat(Integer) (Variables|Default|GetPoints)))) 0.0)
    (Variables|Default|SetPoints (Math|Float|Truncate (Math|Float|Sqrt (Math|Conversions|ToFloat(Integer) (Variables|Default|GetPoints)))))
    (CallFunction|RefreshPoints)
    (else
      (Variables|Default|SetDead? true)
      (CallFunction|GameOver))))

(event Custom|Aumentar%20Puntuacion
  (if (== (Math|Float|Fraction (Math|Float|Sqrt (Math|Conversions|ToFloat(Integer) (Variables|Default|GetPoints)))) 0.0)
    (Variables|Default|SetPoints (Math|Float|Truncate (Math|Float|Power (+ (Math|Float|Sqrt (Math|Conversions|ToFloat(Integer) (Variables|Default|GetPoints))) 1.0) 2.0)))
    (CallFunction|RefreshPoints)
    (else
      (Variables|Default|SetPoints (Math|Float|Truncate (Math|Float|Power (Math|Conversions|ToFloat(Integer) (Variables|Default|GetPoints)) 2.0)))
      (CallFunction|RefreshPoints))))

(event Custom|Game%20Over
  (bind _returnvalue (Game|GetPlayerController 0))
  (Utilities|FlowControl|Delay 1.0)
  (bind _returnvalue_2 (UserInterface|CreateWidget "/Game/Blueprints/Interface/Widgets/W_Fade.W_Fade_C"))
  (Default|FadeOut _returnvalue_2)
  (Utilities|FlowControl|Delay 1.2)
  (bind _returnvalue_3 (UserInterface|CreateWidget "/Game/Blueprints/Interface/Widgets/W_GameOver.W_GameOver_C"))
  (UserInterface|Viewport|AddtoViewport _returnvalue_3 0)
  (Input|SetInputModeGameandUI _returnvalue 0 "DoNotLock" true)
  (Variables|/Script/Engine.PlayerController|SetbShowMouseCursor _returnvalue true))

(event EventBeginPlay
  (bind _outactors (Actor|GetAllActorsOfClass "/Game/Assets_Julia/Blueprints/GridControl.GridControl_C"))
  (bind _output_get (Variables|Default|SetGridReference (Utilities|Array|Get(acopy) _outactors)))
  (Variables|Default|SetGridSize (Variables|/Game/Assets_Julia/Blueprints/GridControl.GridControl_C|GetGridX _output_get))
  (CallFunction|RefreshPoints)
  (Utilities|FlowControl|Delay 0.1)
  (Transformation|SetWorldLocation (Variables|Default|GetCube) (Math|Vector|MakeVector (.x (Transformation|GetWorldLocation (Variables|/Script/Engine.Actor|GetRootComponent (Utilities|Array|Get(acopy) (Variables|/Game/Assets_Julia/Blueprints/GridControl.GridControl_C|GetGridActorMatrix _output_get))))) (.y (Transformation|GetWorldLocation (Variables|/Script/Engine.Actor|GetRootComponent (Utilities|Array|Get(acopy) (Variables|/Game/Assets_Julia/Blueprints/GridControl.GridControl_C|GetGridActorMatrix _output_get))))) (+ (.z (Transformation|GetWorldLocation (Variables|/Script/Engine.Actor|GetRootComponent (Utilities|Array|Get(acopy) (Variables|/Game/Assets_Julia/Blueprints/GridControl.GridControl_C|GetGridActorMatrix _output_get))))) (Variables|Default|GetZ))) false false))

(event Input|ActionEvents|InputActionDown
  (params (Key :type Key%20Structure :default "None"))
  (bind _gridreference (Variables|Default|GetGridReference))
  (bind _gridactormatrix (Variables|/Game/Assets_Julia/Blueprints/GridControl.GridControl_C|GetGridActorMatrix _gridreference))
  (:Pressed
    (Utilities|FlowControl|DoOnce false :!label _label
      (:Completed
        (if (not (Variables|Default|GetDead?))
          (if (Utilities|Array|IsValidIndex _gridactormatrix (+ (Variables|Default|GetTiles%20index) (Variables|Default|GetGridSize)))
            (bind _output_get (Variables|Default|SetTiles%20index (+ (Variables|Default|GetTiles%20index) (Variables|Default|GetGridSize))))
            (Transformation|SetWorldLocation (Variables|Default|GetCube) (Math|Vector|MakeVector (.x (Transformation|GetWorldLocation (Variables|/Script/Engine.Actor|GetRootComponent (Utilities|Array|Get(acopy) _gridactormatrix _output_get)))) (.y (Transformation|GetWorldLocation (Variables|/Script/Engine.Actor|GetRootComponent (Utilities|Array|Get(acopy) _gridactormatrix _output_get)))) (+ (.z (Transformation|GetWorldLocation (Variables|/Script/Engine.Actor|GetRootComponent (Utilities|Array|Get(acopy) _gridactormatrix _output_get)))) (Variables|Default|GetZ))) false false))))))
  (:Released
    (goto _label Reset)))

(event Input|ActionEvents|InputActionUp
  (params (Key :type Key%20Structure :default "None"))
  (bind _gridreference (Variables|Default|GetGridReference))
  (bind _gridactormatrix (Variables|/Game/Assets_Julia/Blueprints/GridControl.GridControl_C|GetGridActorMatrix _gridreference))
  (:Pressed
    (Utilities|FlowControl|DoOnce false :!label _label
      (:Completed
        (if (not (Variables|Default|GetDead?))
          (if (Utilities|Array|IsValidIndex _gridactormatrix (- (Variables|Default|GetTiles%20index) (Variables|Default|GetGridSize)))
            (bind _output_get (Variables|Default|SetTiles%20index (- (Variables|Default|GetTiles%20index) (Variables|Default|GetGridSize))))
            (Transformation|SetWorldLocation (Variables|Default|GetCube) (Math|Vector|MakeVector (.x (Transformation|GetWorldLocation (Variables|/Script/Engine.Actor|GetRootComponent (Utilities|Array|Get(acopy) _gridactormatrix _output_get)))) (.y (Transformation|GetWorldLocation (Variables|/Script/Engine.Actor|GetRootComponent (Utilities|Array|Get(acopy) _gridactormatrix _output_get)))) (+ (.z (Transformation|GetWorldLocation (Variables|/Script/Engine.Actor|GetRootComponent (Utilities|Array|Get(acopy) _gridactormatrix _output_get)))) (Variables|Default|GetZ))) false false))))))
  (:Released
    (goto _label Reset)))

(event Input|ActionEvents|InputActionLeft
  (params (Key :type Key%20Structure :default "None"))
  (bind _gridreference (Variables|Default|GetGridReference))
  (bind _gridactormatrix (Variables|/Game/Assets_Julia/Blueprints/GridControl.GridControl_C|GetGridActorMatrix _gridreference))
  (:Pressed
    (Utilities|FlowControl|DoOnce false :!label _label
      (:Completed
        (if (not (Variables|Default|GetDead?))
          (if (and (Utilities|Array|IsValidIndex _gridactormatrix (+ (Variables|Default|GetTiles%20index) 1)) (!= (Math|Integer|%(Integer) (+ (Variables|Default|GetTiles%20index) 1) (Variables|Default|GetGridSize)) 0))
            (bind _output_get (Variables|Default|SetTiles%20index (+ (Variables|Default|GetTiles%20index) 1)))
            (Transformation|SetWorldLocation (Variables|Default|GetCube) (Math|Vector|MakeVector (.x (Transformation|GetWorldLocation (Variables|/Script/Engine.Actor|GetRootComponent (Utilities|Array|Get(acopy) _gridactormatrix _output_get)))) (.y (Transformation|GetWorldLocation (Variables|/Script/Engine.Actor|GetRootComponent (Utilities|Array|Get(acopy) _gridactormatrix _output_get)))) (+ (.z (Transformation|GetWorldLocation (Variables|/Script/Engine.Actor|GetRootComponent (Utilities|Array|Get(acopy) _gridactormatrix _output_get)))) (Variables|Default|GetZ))) false false))))))
  (:Released
    (goto _label Reset)))

(event Input|ActionEvents|InputActionRight
  (params (Key :type Key%20Structure :default "None"))
  (bind _gridreference (Variables|Default|GetGridReference))
  (bind _gridactormatrix (Variables|/Game/Assets_Julia/Blueprints/GridControl.GridControl_C|GetGridActorMatrix _gridreference))
  (:Pressed
    (Utilities|FlowControl|DoOnce false :!label _label
      (:Completed
        (if (not (Variables|Default|GetDead?))
          (if (and (Utilities|Array|IsValidIndex _gridactormatrix (- (Variables|Default|GetTiles%20index) 1)) (!= (Math|Integer|%(Integer) (Variables|Default|GetTiles%20index) (Variables|Default|GetGridSize)) 0))
            (bind _output_get (Variables|Default|SetTiles%20index (- (Variables|Default|GetTiles%20index) 1)))
            (Transformation|SetWorldLocation (Variables|Default|GetCube) (Math|Vector|MakeVector (.x (Transformation|GetWorldLocation (Variables|/Script/Engine.Actor|GetRootComponent (Utilities|Array|Get(acopy) _gridactormatrix _output_get)))) (.y (Transformation|GetWorldLocation (Variables|/Script/Engine.Actor|GetRootComponent (Utilities|Array|Get(acopy) _gridactormatrix _output_get)))) (+ (.z (Transformation|GetWorldLocation (Variables|/Script/Engine.Actor|GetRootComponent (Utilities|Array|Get(acopy) _gridactormatrix _output_get)))) (Variables|Default|GetZ))) false false))))))
  (:Released
    (goto _label Reset)))

(fn ConstructionScript)

(fn RefreshPoints
  (bind _points (Variables|Default|GetPoints))
  (bind _returnvalue (Utilities|Text|ToText(Integer) _points))
  (Rendering|Components|TextRender|SetText (Variables|Default|GetTextRender1) _returnvalue)
  (Rendering|Components|TextRender|SetText (Variables|Default|GetTextRender2) _returnvalue)
  (Rendering|Components|TextRender|SetText (Variables|Default|GetTextRender) _returnvalue))

(fn GetHUDRef
  (Variables|Components|GetPlayer%20HUD
    (:then
      _)
    (:else
      (Variables|Components|SetPlayer%20HUD (HUD|GetHUD (Game|GetPlayerController 0)))))
  (return (Variables|Components|GetPlayer%20HUD)))