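; BP_Grid is an actor that builds a two-dimensional grid of static mesh tiles when play begins.
; Nested loops over GridX and GridY add one scaled-down static mesh component per cell, placed on the relative X/Y plane using SpacingX and SpacingY.
; Each component is stored in the Tiles array.
; The construction script is empty, so this logic generates tiles only at runtime.
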(event EventBeginPlay
  (for _index (range 0 (Variables|Default|GetGrid%20X))
    (for _index_2 (range 0 (Variables|Default|GetGrid%20Y))
      (bind _returnvalue (AddComponent|AddStaticMeshComponent false (Math|Transform|MakeTransform (Math|Vector|MakeVector (* _index (Variables|Default|GetSpacing%20X)) (* _index_2 (Variables|Default|GetSpacing%20Y)) 0.0) "0, 0, 0" "0.300000,0.300000,0.300000")))
      (Utilities|Array|Add (Variables|Default|GetTiles) _returnvalue))))

(event Collision|EventActorBeginOverlap
  (params (OtherActor :type Actor%20Object%20Reference)))

(event EventTick
  (params (DeltaSeconds :type Float%20%28single-precision%29)))

(fn ConstructionScript)