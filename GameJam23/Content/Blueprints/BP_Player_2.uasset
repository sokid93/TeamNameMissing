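; Player Blueprint for a grid-based number puzzle, moving a cube between BP_Grid tiles and showing Points on three text renders.
; Directional inputs step TilesIndex across a four-wide grid with bounds checks, one move per press.
; AplicarRaiz, also run shortly after BeginPlay, square-roots perfect-square Points, otherwise kills the player, triggering fade and game-over widget.
; AumentarPuntuacion raises perfect squares to the next square and squares other values.
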(event Custom|Aplicar%20Raiz
  (if (== (Math|Float|Fraction (Math|Float|Sqrt (Math|Conversions|ToFloat(Integer) (Variables|Default|GetPoints)))) 0.0)
    (Variables|Default|SetPoints (Math|Float|Truncate (Math|Float|Sqrt (Math|Conversions|ToFloat(Integer) (Variables|Default|GetPoints)))))
    (CallFunction|RefreshPoints)
    (else
      (Variables|Default|SetDead? true)
      (CallFunction|GameOver))))

(event Custom|Aumentar%20Puntuacion
  (if (== (Math|Float|Fraction (Math|Float|Sqrt (Math|Conversions|ToFloat(Integer) (Variables|Default|GetPoints)))) 0.0)
    (Variables|Default|SetPoints (Math|Float|Truncate (Math|Float|Power (+ (Math|Float|Sqrt (Math|Conversions|ToFloat(Integer) (Variables|Default|GetPoints))) 1.0) 2.0)))
    (CallFunction|RefreshPoints)
    (else
      (Variables|Default|SetPoints (Math|Float|Truncate (Math|Float|Power (Math|Conversions|ToFloat(Integer) (Variables|Default|GetPoints)) 2.0)))
      (CallFunction|RefreshPoints))))

(event Custom|Game%20Over
  (bind _returnvalue (Game|GetPlayerController 0))
  (Utilities|FlowControl|Delay 1.0)
  (bind _returnvalue_2 (UserInterface|CreateWidget "/Game/Blueprints/Interface/Widgets/W_Fade.W_Fade_C"))
  (Default|FadeOut _returnvalue_2)
  (Utilities|FlowControl|Delay 1.2)
  (bind _returnvalue_3 (UserInterface|CreateWidget "/Game/Blueprints/Interface/Widgets/W_GameOver.W_GameOver_C"))
  (UserInterface|Viewport|AddtoViewport _returnvalue_3 0)
  (Input|SetInputModeGameandUI _returnvalue 0 "DoNotLock" true)
  (Variables|/Script/Engine.PlayerController|SetbShowMouseCursor _returnvalue true))

(event EventBeginPlay
  (CallFunction|RefreshPoints)
  (Utilities|FlowControl|Delay 0.1)
  (Transformation|SetWorldLocation (Variables|Default|GetCube) (Transformation|GetWorldLocation (Utilities|Array|Get(acopy) (Variables|/Game/Blueprints/BP_Grid.BP_Grid_C|GetTiles (CallFunction|GetGridRef)))) false false)
  (Utilities|FlowControl|Delay 1.2)
  (CallFunction|AplicarRaiz))

(event Input|ActionEvents|InputActionDown
  (params (Key :type Key%20Structure :default "None"))
  (bind _output_get (CallFunction|GetGridRef))
  (bind _tiles (Variables|/Game/Blueprints/BP_Grid.BP_Grid_C|GetTiles _output_get))
  (:Pressed
    (Utilities|FlowControl|DoOnce false :!label _label
      (:Completed
        (if (not (Variables|Default|GetDead?))
          (if (Utilities|Array|IsValidIndex _tiles (+ (Variables|Default|GetTiles%20index) 4))
            (bind _output_get_2 (Variables|Default|SetTiles%20index (+ (Variables|Default|GetTiles%20index) 4)))
            (Transformation|SetWorldLocation (Variables|Default|GetCube) (Transformation|GetWorldLocation (Utilities|Array|Get(acopy) _tiles _output_get_2)) false false))))))
  (:Released
    (goto _label Reset)))

(event Input|ActionEvents|InputActionUp
  (params (Key :type Key%20Structure :default "None"))
  (bind _output_get (CallFunction|GetGridRef))
  (bind _tiles (Variables|/Game/Blueprints/BP_Grid.BP_Grid_C|GetTiles _output_get))
  (:Pressed
    (Utilities|FlowControl|DoOnce false :!label _label
      (:Completed
        (if (not (Variables|Default|GetDead?))
          (if (Utilities|Array|IsValidIndex _tiles (- (Variables|Default|GetTiles%20index) 4))
            (bind _output_get_2 (Variables|Default|SetTiles%20index (- (Variables|Default|GetTiles%20index) 4)))
            (Transformation|SetWorldLocation (Variables|Default|GetCube) (Transformation|GetWorldLocation (Utilities|Array|Get(acopy) _tiles _output_get_2)) false false))))))
  (:Released
    (goto _label Reset)))

(event Input|ActionEvents|InputActionLeft
  (params (Key :type Key%20Structure :default "None"))
  (bind _output_get (CallFunction|GetGridRef))
  (bind _tiles (Variables|/Game/Blueprints/BP_Grid.BP_Grid_C|GetTiles _output_get))
  (:Pressed
    (Utilities|FlowControl|DoOnce false :!label _label
      (:Completed
        (if (not (Variables|Default|GetDead?))
          (if (and (Utilities|Array|IsValidIndex _tiles (+ (Variables|Default|GetTiles%20index) 1)) (!= (Math|Integer|%(Integer) (+ (Variables|Default|GetTiles%20index) 1) 4) 0))
            (bind _output_get_2 (Variables|Default|SetTiles%20index (+ (Variables|Default|GetTiles%20index) 1)))
            (Transformation|SetWorldLocation (Variables|Default|GetCube) (Transformation|GetWorldLocation (Utilities|Array|Get(acopy) _tiles _output_get_2)) false false))))))
  (:Released
    (goto _label Reset)))

(event Input|ActionEvents|InputActionRight
  (params (Key :type Key%20Structure :default "None"))
  (bind _output_get (CallFunction|GetGridRef))
  (bind _tiles (Variables|/Game/Blueprints/BP_Grid.BP_Grid_C|GetTiles _output_get))
  (:Pressed
    (Utilities|FlowControl|DoOnce false :!label _label
      (:Completed
        (if (not (Variables|Default|GetDead?))
          (if (and (Utilities|Array|IsValidIndex _tiles (- (Variables|Default|GetTiles%20index) 1)) (!= (Math|Integer|%(Integer) (Variables|Default|GetTiles%20index) 4) 0))
            (bind _output_get_2 (Variables|Default|SetTiles%20index (- (Variables|Default|GetTiles%20index) 1)))
            (Transformation|SetWorldLocation (Variables|Default|GetCube) (Transformation|GetWorldLocation (Utilities|Array|Get(acopy) _tiles _output_get_2)) false false))))))
  (:Released
    (goto _label Reset)))

(fn ConstructionScript)

(fn RefreshPoints
  (bind _points (Variables|Default|GetPoints))
  (bind _returnvalue (Utilities|Text|ToText(Integer) _points))
  (Rendering|Components|TextRender|SetText (Variables|Default|GetTextRender1) _returnvalue)
  (Rendering|Components|TextRender|SetText (Variables|Default|GetTextRender2) _returnvalue)
  (Rendering|Components|TextRender|SetText (Variables|Default|GetTextRender) _returnvalue))

(fn GetGridRef
  (bind _returnvalue (Actor|GetActorOfClass "/Game/Blueprints/BP_Grid.BP_Grid_C"))
  (bind _output_get (Variables|Default|SetGrid%20Ref _returnvalue))
  (return _output_get))

(fn GetHUDRef
  (Variables|Default|GetPlayer%20HUD
    (:then
      _)
    (:else
      (Variables|Default|SetPlayer%20HUD (HUD|GetHUD (Game|GetPlayerController 0)))))
  (return (Variables|Default|GetPlayer%20HUD)))